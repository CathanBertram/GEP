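; Purchasable weapon stand prop with a child actor weapon and a text socket, built for a rotating display until unlocked.
; A Rotate timeline update sets the yaw of both sockets and bobs the weapon along its relative Y axis, stopping once Unlocked is true.
; Nothing in the graph starts the timeline, so this animation never runs.
; The file holds no purchase logic, and the construction script is empty.
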(fn `UserConstructionScript`)