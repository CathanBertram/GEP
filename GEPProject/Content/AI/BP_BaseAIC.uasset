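; Base AI controller that runs a supplied behavior tree and tracks sight of a single target pawn.
; SetupAIC stores the tree and target, then seeds the Blackboard with Target and the controlled pawn's location as Origin.
; When PawnSensing sees the target, it sets CanSeeTarget and RecentlySeenTarget.
; A retriggerable delay of twice the sensing interval clears CanSeeTarget once sightings stop; RecentlySeenTarget is never cleared here.
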(event `SetupAIC`
  (params (BehaviourTree :type "BehaviorTree Object Reference") (PawnSensingTarget :type "Pawn Object Reference"))
  (bind _pawnsensingtarget (`self.PawnSensingTarget`))
  (set `self.BehaviourTree` BehaviourTree)
  (set `self.PawnSensingTarget` PawnSensingTarget)
  (`self.RunBehaviorTree` (`self.BehaviourTree`))
  (`/Game/AI/AIFunctionLibrary.UpdateBBKey` self "Target" true "NewEnumerator1" _pawnsensingtarget)
  (`/Game/AI/AIFunctionLibrary.UpdateBBKey` self "Origin" false "NewEnumerator2" _pawnsensingtarget (`self.K2_GetActorLocation` (`self.K2_GetPawn`))))

(event `self.PawnSensing.OnSeePawn`
  (params (Pawn :type "Pawn Object Reference"))
  (if (== Pawn (`self.PawnSensingTarget`))
    (`|ExecutionSequence`
      (:`then_0`
        (`/Game/AI/AIFunctionLibrary.UpdateBBKey` self "CanSeeTarget" true)
        (`KismetSystemLibrary.RetriggerableDelay` (* (`PawnSensingComponent.SensingInterval` (`self.PawnSensing`)) 2.0))
        (`/Game/AI/AIFunctionLibrary.UpdateBBKey` self "CanSeeTarget"))
      (:`then_1`
        (`/Game/AI/AIFunctionLibrary.UpdateBBKey` self "RecentlySeenTarget" true)))))

(fn `UserConstructionScript`)