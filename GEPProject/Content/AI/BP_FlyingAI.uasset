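; BP_FlyingAI is an AI-controlled flying pawn that hands its behaviour to a BP_BaseAIC controller.
; On BeginPlay it turns off controller-driven rotation and orients the character to its movement direction.
; It then casts its AI controller and calls SetupAIC with its behaviour tree, the player pawn as sensing target, and its move-to parameters.
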(event `self.ReceiveBeginPlay`
  (set `self.bUseControllerRotationPitch` false)
  (set `self.bUseControllerRotationRoll` false)
  (set `self.bUseControllerRotationYaw` false)
  (set `CharacterMovementComponent.bOrientRotationToMovement` true (`self.CharacterMovement`))
  (bind _asbp_base_aic (cast `/Game/AI/BP_BaseAIC` (`AIBlueprintHelperLibrary.GetAIController` self))) ; CHANGE CAST
  (`/Game/AI/BP_BaseAIC.SetupAIC` _asbp_base_aic (`self.BehaviourTree`) (`GameplayStatics.GetPlayerPawn` 0) (`self.BP_AIMoveToParameters`)))

(fn `UserConstructionScript`)