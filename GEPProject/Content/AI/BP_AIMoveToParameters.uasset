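; BP_AIMoveToParameters configures its owning Character for damped, gravity-free physics movement, apparently for AI movement.
; Setup casts the owner to Character, caches it and its capsule, enables capsule physics simulation, disables gravity on capsule and movement component, and applies linear and angular damping.
; The cast branches appear inverted: success only prints a "no character" message, while the configuration runs on failure.
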(event `Setup`
  (bind _physicscapsuleref (`self.PhysicsCapsuleRef`))
  (bind _physicscapsuleref_2 (`self.PhysicsCapsuleRef`))
  (bind _ascharacter (cast `Character` (`self.GetOwner`)) ; Replace dogshit cast ew icky wicky
    (:`then`
      (`KismetSystemLibrary.PrintString` "no character dumb dumb"))
    (:`CastFailed`
      (bind _output_get (set `self.OwningCharRef` _ascharacter))
      (set `self.PhysicsCapsuleRef` (`Character.CapsuleComponent` _output_get))
      (`PrimitiveComponent.SetSimulatePhysics` _physicscapsuleref_2 true)
      (`PrimitiveComponent.SetEnableGravity` _physicscapsuleref_2 false)
      (set `CharacterMovementComponent.GravityScale` 0.0 (`Character.CharacterMovement` (`self.OwningCharRef`)))
      (`PrimitiveComponent.SetLinearDamping` _physicscapsuleref (`self.LinearDamping`))
      (`PrimitiveComponent.SetAngularDamping` _physicscapsuleref (`self.AngularDamping`)))))