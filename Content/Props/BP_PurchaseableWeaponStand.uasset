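; Purchasable weapon stand prop, built to display a rotating, bobbing weapon and text until it is unlocked.
; A Rotate timeline drives the yaw of the weapon and text sockets and offsets the weapon child actor along relative Y, stopping once Unlocked is set.
; Nothing in the graph starts that timeline, and no purchase or unlock logic is present.
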(fn `UserConstructionScript`)